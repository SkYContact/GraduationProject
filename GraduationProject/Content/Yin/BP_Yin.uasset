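; BP_Yin is a player-controllable character with axis movement, jumping and foot IK.
; Each tick it passes left and right foot socket names to GetIKFootLocation with a trace distance, raises the results by a fixed Z offset, and writes them to ABP_Yin.
; Movement follows the actor's forward and right vectors.
; A CanJumpInternal override permits jumping only while the actor is below a fixed world height, without checking for ground contact.
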(event `self.ReceiveBeginPlay`
  (bind _asabp_yin (cast `/Game/Yin/ABP_Yin` (`SkeletalMeshComponent.GetAnimInstance` (`self.Mesh`))))
  (set `self.As ABP Yin` _asabp_yin))

(event `self.ReceiveTick`
  (params (DeltaSeconds :type "Float (single-precision)"))
  (bind _ikfootlocation (`self.Get Foot IKLocation` (`/Game/Yin/ABP_Yin.LeftIKFoot Socket Name` (`self.As ABP Yin`))))
  (set `/Game/Yin/ABP_Yin.LeftIKFootLocation` _ikfootlocation (`self.As ABP Yin`))
  (bind _ikfootlocation_2 (`self.Get Foot IKLocation` (`/Game/Yin/ABP_Yin.RightIKFoot Socket Name` (`self.As ABP Yin`))))
  (set `/Game/Yin/ABP_Yin.RightIKFootLocation` _ikfootlocation_2 (`self.As ABP Yin`)))

(event `InputAxis|MoveUp`
  (params (AxisValue :type "Float (single-precision)"))
  (`self.AddMovementInput` (`self.GetActorForwardVector`) AxisValue))

(event `InputAxis|MoveRight`
  (params (AxisValue :type "Float (single-precision)"))
  (`self.AddMovementInput` (`self.GetActorRightVector`) AxisValue))

(event `InputAction|Jump`
  (params (Key :type "Key Structure"))
  (:`Pressed`
    (`self.Jump`)))

(fn `CanJumpInternal`
  (returns (ReturnValue :type Boolean))
  (bind (_returnvalue_x _returnvalue_y _returnvalue_z) (`KismetMathLibrary.BreakVector` (`self.K2_GetActorLocation`)))
  (return (< _returnvalue_z 300.0)))

(fn `Get Foot IKLocation`
  (params (`FKFoot Socket Name` :type Name))
  (returns (IKFootLocation :type "Vector Structure"))
  (bind _returnvalue (`self.GetIKFootLocation` (`self.Foot IKTrace Distance`) `FKFoot Socket Name` (`self.IKRoot Socket Name`)))
  (return (`KismetMathLibrary.MakeVector` (.x _returnvalue) (.y _returnvalue) (+ (.z _returnvalue) 15.0))))

(fn `UserConstructionScript`)